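; Player character for a Pac-Man-style game that tracks score, lives and a temporary super power.
; It counts Coin actors on BeginPlay; IncrementScore calls WinGame at that total, which disables input and shows the win widget.
; DecreaseLives is skipped while invincible; at zero it freezes movement, shows Game Over and asks PacmanGameMode to restart.
; SetSuperPower grants speed and invincibility, then reverts both after a delay.
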(event Custom|SetSuperPower
  (CallFunction|SuperPower)
  (Utilities|FlowControl|Delay 5.0)
  (Variables|Default|SetbIsInvencible false)
  (Variables|/Script/Engine.CharacterMovementComponent|SetMaxWalkSpeed (Variables|Character|GetCharacterMovement) 1.2e+03))

(event Custom|WinGame
  (Components|Movement|StopMovementImmediately (Variables|Character|GetCharacterMovement))
  (Variables|Default|SetbIsInvencible true)
  (Input|DisableInput (Game|GetPlayerController 0))
  (bind _returnvalue (UserInterface|CreateWidget "/Game/UI/WinGame.WinGame_C"))
  (UserInterface|Viewport|AddtoViewport _returnvalue 0))

(event EventBeginPlay
  (bind _outactors (Actor|GetAllActorsOfClass "/Game/Blueprints/Coin.Coin_C"))
  (Variables|Default|SetTotalCoins (Utilities|Array|Length _outactors)))

(event Collision|EventActorBeginOverlap
  (params (OtherActor :type Actor%20Object%20Reference)))

(event EventTick
  (params (DeltaSeconds :type Float%20%28single-precision%29)))

(event Input|AxisEvents|InputAxisForwardMovement
  (params (AxisValue :type Float%20%28single-precision%29))
  (Pawn|Input|AddMovementInput (Transformation|GetActorForwardVector) AxisValue false))

(event Input|AxisEvents|InputAxisRightwardMovement
  (params (AxisValue :type Float%20%28single-precision%29))
  (Pawn|Input|AddMovementInput (Transformation|GetActorRightVector) AxisValue false))

(fn ConstructionScript)

(fn IncrementScore
  (bind _result (Math|Integer|IncrementInt (Variables|Default|GetScore))
    (:%20%20
      (if (>= _result (Variables|Default|GetTotalCoins))
        (CallFunction|WinGame)))))

(fn IncrementLives
  (Math|Integer|IncrementInt (Variables|Default|GetLives)))

(fn DecreaseLives
  (bind _charactermovement (Variables|Character|GetCharacterMovement))
  (if (not (Variables|Default|GetbIsInvencible))
    (bind _result (Math|Integer|DecrementInt (Variables|Default|GetLives))
      (:%20%20
        (if (<= _result 0)
          (Variables|Default|SetLives 0)
          (Components|Movement|StopMovementImmediately _charactermovement)
          (Pawn|Components|CharacterMovement|SetMovementMode _charactermovement "MOVE_None" 0)
          (bind _returnvalue (UserInterface|CreateWidget "/Game/UI/GameOver.GameOver_C"))
          (UserInterface|Viewport|AddtoViewport _returnvalue 0)
          (bind _aspacman_game_mode (Utilities|Casting|CastToPacmanGameMode (Game|GetGameMode)))
          (Default|RestartLevel _aspacman_game_mode))))))

(fn SuperPower
  (Variables|/Script/Engine.CharacterMovementComponent|SetMaxWalkSpeed (Variables|Character|GetCharacterMovement) 3e+03)
  (Variables|Default|SetbIsInvencible true))