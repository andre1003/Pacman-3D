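; Ghost enemy that wanders between random TargetPoints in the level and costs the Player a life on overlap.
; After a start delay, it AI-moves at its own height to a random point, picking another on arrival or via a fallback timer.
; Overlapping an invincible Player spawns a fresh Ghost at its initial transform and destroys itself; otherwise it decreases lives and shows a Damage widget.
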(event EventBeginPlay
  (bind _self self)
  (Variables|Default|SetInitialTransform (Transformation|GetActorTransform))
  (bind _outactors (Actor|GetAllActorsOfClass "/Script/Engine.TargetPoint"))
  (bind _output_get (Variables|Default|SetTargetPoints _outactors))
  (Utilities|FlowControl|Delay (Variables|Default|GetStartDelay))
  (bind _output_get_2 (Variables|Default|SetCurrentTargetPointIndex (Math|Random|RandomIntegerinRange 0 (- (Utilities|Array|Length _output_get) 1)) :!label _label))
  (AI|AIMoveTo _self (Math|Vector|MakeVector (.x (Transformation|GetActorLocation (Utilities|Array|Get(acopy) _output_get _output_get_2))) (.y (Transformation|GetActorLocation (Utilities|Array|Get(acopy) _output_get _output_get_2))) (.z (Transformation|GetActorLocation _self))) 0 5.0 false
    (:then
      (Utilities|FlowControl|Delay 25.0)
      (goto _label))
    (:OnSuccess
      (goto _label))))

(event Collision|EventActorBeginOverlap
  (params (OtherActor :type Actor%20Object%20Reference))
  (bind _asplayer (Utilities|Casting|CastToPlayer OtherActor))
  (if (Variables|/Game/Blueprints/Player.Player_C|GetbIsInvencible _asplayer)
    (Game|SpawnActorfromClass "Ghost_C" (Variables|Default|GetInitialTransform) "Undefined" 0 0)
    (Actor|DestroyActor)
    (else
      (Default|DecreaseLives _asplayer)
      (bind _returnvalue (UserInterface|CreateWidget "/Game/UI/Damage.Damage_C"))
      (UserInterface|Viewport|AddtoViewport _returnvalue 0))))

(event EventTick
  (params (DeltaSeconds :type Float%20%28single-precision%29)))

(fn ConstructionScript)